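; Rhino fish enemy that attacks the player with a ranged roll charge and a close-range bite.
; A looping timer checks range and line of sight, then starts a timed, invulnerable roll toward the player that damages on capsule contact.
; Entering the bite collision swaps searching for a repeating bite with animation-delayed damage, which takes priority over rolling.
; Both attacks aim at the player, flipping the sprite by yaw, and swap flipbooks.
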(event OnComponentBeginOverlap(CapsuleComponent)
  (params (OverlappedComponent :type Primitive%20Component%20Object%20Reference) (OtherActor :type Actor%20Object%20Reference) (OtherComp :type Primitive%20Component%20Object%20Reference) (OtherBodyIndex :type Integer) (bFromSweep :type Boolean) (SweepResult :type Hit%20Result%20Structure%20%28by%20ref%29))
  (if (Variables|Cached|GetIsRolling)
    (bind _asmech_paper_player (Utilities|Casting|CastToMechPaperPlayer OtherActor))
    (Class|MechPaperDroid|TakeDamage _asmech_paper_player (Variables|Config|GetRollDamage))))

(event OnComponentBeginOverlap(BiteCollision)
  (params (OverlappedComponent :type Primitive%20Component%20Object%20Reference) (OtherActor :type Actor%20Object%20Reference) (OtherComp :type Primitive%20Component%20Object%20Reference) (OtherBodyIndex :type Integer) (bFromSweep :type Boolean) (SweepResult :type Hit%20Result%20Structure%20%28by%20ref%29))
  (Utilities|Casting|CastToMechPaperPlayer OtherActor)
  (if (not (or (Variables|Cached|GetIsBiting) (Variables|Cached|GetIsRolling)))
    (Utilities|Time|ClearTimerbyFunctionName 0 (Variables|Cached|GetSearchForPlayerFunctionName))
    (bind _returnvalue (Utilities|Time|SetTimerbyEvent (delegate Custom|Bite) 0.1 true))
    (Variables|Cached|SetBiteTimer _returnvalue)))

(event OnComponentEndOverlap(BiteCollision)
  (params (OverlappedComponent :type Primitive%20Component%20Object%20Reference) (OtherActor :type Actor%20Object%20Reference) (OtherComp :type Primitive%20Component%20Object%20Reference) (OtherBodyIndex :type Integer))
  (Utilities|Casting|CastToMechPaperPlayer OtherActor)
  (if (not (Variables|Cached|GetIsRolling))
    (Utilities|Time|ClearandInvalidateTimerbyHandle (Variables|Cached|GetBiteTimer))
    (Utilities|Time|SetTimerbyFunctionName 0 (Variables|Cached|GetSearchForPlayerFunctionName) 2.0 true)))

(event Custom|Bite
  (bind _sprite (Variables|Default|GetSprite))
  (bind _sprite_2 (Variables|Default|GetSprite))
  (Utility|SetDirection)
  (Variables|Cached|SetIsBiting true)
  (Sprite|SetFlipbook _sprite_2 "/Game/Textures/Droids/Warped_Rino_Fish/rino-fish-bite/sprites/FB_Rino-Fish_Bite.FB_Rino-Fish_Bite")
  (Components|Timeline|SetLooping _sprite_2 false)
  (Utilities|FlowControl|Delay 0.15) ; Delay damage for animation
  (Attack|BitePlayer)
  (Utilities|FlowControl|Delay (Class|PaperFlipbookComponent|GetFlipbookLength _sprite_2))
  (Sprite|SetFlipbook _sprite "/Game/Textures/Droids/Warped_Rino_Fish/rino-fish-idle/sprites/FB_Rino-Fish_Idle.FB_Rino-Fish_Idle")
  (Components|Timeline|SetLooping _sprite true)
  (Audio|Components|Audio|Play _sprite)
  (Variables|Cached|SetIsBiting false))

(event Custom|Roll
  (Utility|SetDirection)
  (Utilities|FlowControl|Delay 0.5)
  (if (not (Variables|Cached|GetIsBiting)) ; Give Bite higher priority to avoid issues
    (Variables|Cached|SetIsRolling true)
    (Attack|StartRolling)
    (Utilities|FlowControl|Delay 2.0)
    (Attack|StopRolling)
    (Variables|Cached|SetIsRolling false)))

(event EventTick
  (params (DeltaSeconds :type Float%20%28single-precision%29))
  (if (Variables|Cached|GetIsRolling)
    (Pawn|Input|AddMovementInput (Variables|Cached|GetRollingDirection) 1.0 false)))

(event EventBeginPlay
  (Utilities|Time|SetTimerbyFunctionName 0 (Variables|Cached|GetSearchForPlayerFunctionName) 2.0 true)
  (EventDispatchers|BindEventtoOnDeath (EventDispatchers|CreateEvent :!event OnDie)))

(fn ConstructionScript)

(fn BitePlayer
  (bind _output_get (LocalVariables|SetLocalPlayers (Collision|GetOverlappingActors (Variables|Default|GetBiteCollision) "/Script/Mechbot.MechPaperPlayer" :!class /Script/Engine.PrimitiveComponent)))
  (for _array_element _output_get
    (bind _asmech_paper_player (Utilities|Casting|CastToMechPaperPlayer _array_element))
    (Class|MechPaperDroid|TakeDamage _asmech_paper_player (Variables|Config|GetBiteDamage))))

(fn StartRolling
  (Sprite|SetFlipbook (Variables|Default|GetSprite) "/Game/Textures/Droids/Warped_Rino_Fish/rino-fish-rolling/sprites/FB_Rino-Fish_Rolling.FB_Rino-Fish_Rolling")
  (Class|MechPaperDroid|SetCanbeDamaged false))

(fn StopRolling
  (Class|NavMovementComponent|StopActiveMovement (Variables|Character|GetCharacterMovement))
  (Sprite|SetFlipbook (Variables|Default|GetSprite) "/Game/Textures/Droids/Warped_Rino_Fish/rino-fish-idle/sprites/FB_Rino-Fish_Idle.FB_Rino-Fish_Idle")
  (Class|MechPaperDroid|SetCanbeDamaged true))

(fn SearchforPlayer
  (if (Math|Boolean|NORBoolean (Variables|Cached|GetIsBiting) (Variables|Cached|GetIsRolling))
    (LocalVariables|SetLocalPlayer (Game|Player|GetPlayerPawn 0))
    (LocalVariables|SetLocalSelfLocation (Transformation|GetActorLocation))
    (LocalVariables|SetLocalPlayerLocation (Transformation|GetActorLocation (LocalVariables|GetLocalPlayer)))
    (if (<= (Math|Vector|Distance(Vector) (LocalVariables|GetLocalSelfLocation) (LocalVariables|GetLocalPlayerLocation)) (Variables|Config|GetSearchRange))
      (bind _outhit (Collision|LineTraceForObjects (LocalVariables|GetLocalSelfLocation) (LocalVariables|GetLocalPlayerLocation) (Utilities|Array|MakeArray "ObjectTypeQuery3") false (Utilities|Array|MakeArray self) "None"))
      (if (== (.HitActor (Collision|BreakHitResult _outhit)) (LocalVariables|GetLocalPlayer))
        (CallFunction|Roll)))))

(fn SetDirection
  (bind _sprite (Variables|Default|GetSprite))
  (bind _output_get (Variables|Cached|SetRollingDirection (Math|Vector|GetUnitDirection(Vector) (Transformation|GetActorLocation) (Transformation|GetActorLocation (Game|Player|GetPlayerPawn 0)))))
  ;[1 1 1] Hacky way to set character mesh based on direction it's facing
  (Math|Float|CompareFloat (- (.Yaw (Math|Vector|GetYawPitchfromVector _output_get)) 5e+01) 0.0
    (:>
      (Transformation|SetWorldRotation _sprite (Math|Rotator|MakeRotator 0.0 0.0 1.8e+02) false false))
    (:<
      (Transformation|SetWorldRotation _sprite (Math|Rotator|MakeRotator 0.0 0.0 0.0) false false))))

(fn OnDie
  (Actor|DestroyActor))