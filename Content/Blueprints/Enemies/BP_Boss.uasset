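; Paper2D bug boss that wakes when the player pawn fires StartBossFight, staying invulnerable and passive during a short intro.
; It walks toward the player, flipping its sprite by yaw, and attacks via a looping timer or AttackRadius overlap.
; SlashAttack teleports it behind the player before enabling the damage collider, with flipbook completion driving the attack cycle.
; Death disables collision and timers, plays a roll animation, then calls the player's win.
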(event OnComponentBeginOverlap(SlashCollision)
  (params (OverlappedComponent :type Primitive%20Component%20Object%20Reference) (OtherActor :type Actor%20Object%20Reference) (OtherComp :type Primitive%20Component%20Object%20Reference) (OtherBodyIndex :type Integer) (bFromSweep :type Boolean) (SweepResult :type Hit%20Result%20Structure%20%28by%20ref%29))
  (bind _asmech_paper_player (Utilities|Casting|CastToMechPaperPlayer OtherActor))
  (Class|MechPaperDroid|TakeDamage _asmech_paper_player (Variables|Default|GetSlashDamage)))

(event OnComponentBeginOverlap(AttackRadius)
  (params (OverlappedComponent :type Primitive%20Component%20Object%20Reference) (OtherActor :type Actor%20Object%20Reference) (OtherComp :type Primitive%20Component%20Object%20Reference) (OtherBodyIndex :type Integer) (bFromSweep :type Boolean) (SweepResult :type Hit%20Result%20Structure%20%28by%20ref%29))
  (Utilities|Casting|CastToMechPaperPlayer OtherActor)
  (if (Class|MechPaperDroid|CanAttack)
    (CallFunction|SlashAttack)))

(event Custom|Die
  (bind _sprite (Variables|Default|GetSprite))
  (Collision|SetCollisionEnabled (Variables|Default|GetCapsuleComponent) "NoCollision")
  (EventDispatchers|UnbindallEventsfromOnFinishedPlaying (Variables|Default|GetSprite))
  (Utilities|Time|ClearandInvalidateTimerbyHandle (Variables|Default|GetAttackTimer))
  (Utilities|Time|ClearTimerbyFunctionName 0 "WalkTowardsPlayer")
  (Components|Timeline|SetLooping _sprite false)
  (Sprite|SetFlipbook _sprite "/Game/Textures/Droids/Bug_Hulk/Flipbooks/FB_Bug_Hulk-Roll.FB_Bug_Hulk-Roll")
  (Components|Timeline|PlayfromStart _sprite)
  (EventDispatchers|BindEventtoOnFinishedPlaying _sprite (delegate Custom|Win)))

(event Custom|Win
  (Utilities|FlowControl|Delay 1.0)
  (bind _asbp_mech_paper_player (Utilities|Casting|CastToBP_MechPaperPlayer (Game|Player|GetPlayerPawn 0)))
  (Default|CallWin _asbp_mech_paper_player))

(event Custom|SlashAttack
  (bind _sprite (Variables|Default|GetSprite))
  (if (Class|MechPaperDroid|CanAttack)
    (Utilities|Time|ClearandInvalidateTimerbyHandle (Variables|Default|GetAttackTimer))
    (Class|MechPaperDroid|SetCanAttack false)
    (Components|Movement|StopMovementImmediately (Variables|Character|GetCharacterMovement))
    (Collision|SetCollisionEnabled (Variables|Default|GetAttackRadius) "NoCollision")
    (Sprite|SetFlipbook _sprite "/Game/Textures/Droids/Bug_Hulk/Flipbooks/FB_Bug_Hulk-Slash.FB_Bug_Hulk-Slash")
    (Components|Timeline|SetLooping _sprite false)
    (Utilities|FlowControl|Delay 0.1)
    (EventDispatchers|BindEventtoOnFinishedPlaying _sprite (EventDispatchers|CreateEvent :!event Custom|Reset))
    (Movement|TeleporttoPlayer)
    (Utilities|FlowControl|Delay 0.3)
    (Collision|SetCollisionEnabled (Variables|Default|GetSlashCollision) "QueryOnly")))

(event Custom|Reset
  (bind _sprite (Variables|Default|GetSprite))
  (Collision|SetCollisionEnabled (Variables|Default|GetSlashCollision) "NoCollision")
  (Sprite|SetFlipbook _sprite "/Game/Textures/Droids/Bug_Hulk/Flipbooks/FB_BugHulk_Walk.FB_BugHulk_Walk")
  (Components|Timeline|SetLooping _sprite true)
  (Components|Timeline|PlayfromStart _sprite)
  (Collision|SetCollisionEnabled (Variables|Default|GetAttackRadius) "QueryOnly")
  (Class|MechPaperDroid|SetCanAttack true)
  (bind _returnvalue (Utilities|Time|SetTimerbyEvent (EventDispatchers|CreateEvent :!event Custom|SlashAttack) 5.0 true))
  (Variables|Default|SetAttackTimer _returnvalue))

(event Custom|BossIntro
  (Class|MechPaperDroid|SetCanAttack false)
  (Class|MechPaperDroid|SetCanbeDamaged false)
  (bind _returnvalue (Utilities|Time|SetTimerbyEvent (EventDispatchers|CreateEvent :!event Custom|SlashAttack) 5.0 true))
  (Variables|Default|SetAttackTimer _returnvalue)
  (Utilities|FlowControl|Delay 3.5)
  (Class|MechPaperDroid|SetCanAttack true)
  (Class|MechPaperDroid|SetCanbeDamaged true)
  (Collision|SetCollisionEnabled (Variables|Default|GetAttackRadius) "QueryOnly")
  (Utilities|Time|SetTimerbyFunctionName 0 "WalkTowardsPlayer" 1.5 true))

(event EventBeginPlay
  (EventDispatchers|BindEventtoOnDeath (EventDispatchers|CreateEvent :!event Custom|Die))
  (bind _asbp_mech_paper_player (Utilities|Casting|CastToBP_MechPaperPlayer (Game|Player|GetPlayerPawn 0)))
  (EventDispatchers|BindEventtoStartBossFight _asbp_mech_paper_player (delegate Custom|BossIntro)))

(event EventTick
  (params (DeltaSeconds :type Float%20%28single-precision%29))
  (if (Class|MechPaperDroid|IsAlive)
    (Movement|WalkTowardsPlayer)))

(fn ConstructionScript)

(fn WalkTowardsPlayer
  (bind _sprite (Variables|Default|GetSprite))
  (if (Class|MechPaperDroid|CanAttack)
    (LocalVariables|SetLocalDirection (Math|Vector|GetUnitDirection(Vector) (Transformation|GetActorLocation) (Transformation|GetActorLocation (Game|Player|GetPlayerPawn 0))))
    (Utilities|FlowControl|Sequence
      (:then_0
        ;[1 1 1] Hacky way to set character mesh based on direction it's facing
        (Math|Float|CompareFloat (- (.Yaw (Math|Vector|GetYawPitchfromVector (LocalVariables|GetLocalDirection))) 5e+01) 0.0
          (:>
            (Transformation|SetWorldRotation _sprite (Math|Rotator|MakeRotator 0.0 0.0 0.0) false false))
          (:<
            (Transformation|SetWorldRotation _sprite (Math|Rotator|MakeRotator 0.0 0.0 1.8e+02) false false))))
      (:then_1
        (Pawn|Input|AddMovementInput (LocalVariables|GetLocalDirection) 1.0 false)))))

(fn TeleporttoPlayer
  (bind _asmech_paper_player (Utilities|Casting|CastToMechPaperPlayer (Game|Player|GetPlayerPawn 0)))
  (LocalVariables|SetLocalLocation (Transformation|GetActorLocation _asmech_paper_player))
  (Transformation|SetActorLocationAndRotation (Math|Vector|MakeVector (+ (.x (LocalVariables|GetLocalLocation)) (.x (* (Transformation|GetActorForwardVector _asmech_paper_player) -3e+01))) (.y (LocalVariables|GetLocalLocation)) (.z (Transformation|GetActorLocation))) (Transformation|GetWorldRotation (Variables|/Script/Paper2D.PaperCharacter|GetSprite _asmech_paper_player)) false true))