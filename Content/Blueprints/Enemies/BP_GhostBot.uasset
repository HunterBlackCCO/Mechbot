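; Paper2D ghost enemy that chases the player and deals contact damage, using Owlet monster flipbooks.
; Each tick picks a jump, walk or idle animation and calls HauntPlayer when a range-limited, Pawn-only trace finds the player or attack is cooling down.
; HauntPlayer steers at the living player, flipping the sprite by yaw, or drifts slowly along its facing during the post-hit cooldown.
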(event OnComponentBeginOverlap(CapsuleComponent)
  (params (OverlappedComponent :type Primitive%20Component%20Object%20Reference) (OtherActor :type Actor%20Object%20Reference) (OtherComp :type Primitive%20Component%20Object%20Reference) (OtherBodyIndex :type Integer) (bFromSweep :type Boolean) (SweepResult :type Hit%20Result%20Structure%20%28by%20ref%29))
  (bind _asmech_paper_player (Utilities|Casting|CastToMechPaperPlayer OtherActor))
  (Class|MechPaperDroid|TakeDamage _asmech_paper_player 20)
  (Class|MechPaperDroid|SetCanAttack false)
  (Utilities|FlowControl|Delay 2.0)
  (Class|MechPaperDroid|SetCanAttack true))

(event Custom|HandleAnimation
  (bind _sprite (Variables|Default|GetSprite))
  (bind _charactermovement (Variables|Character|GetCharacterMovement))
  (if (AI|Components|NavMovement|IsFalling _charactermovement)
    (Sprite|SetFlipbook _sprite "/Game/Textures/Droids/GhostBot/Flipbooks/FB_Owlet_Monster_Jump.FB_Owlet_Monster_Jump")
    (elif (> (Math|Vector|VectorLength (Variables|/Script/Engine.MovementComponent|GetVelocity _charactermovement)) 0.0)
      (Sprite|SetFlipbook _sprite "/Game/Textures/Droids/GhostBot/Flipbooks/FB_Owlet_Monster_Walk.FB_Owlet_Monster_Walk")
      (else
        (Sprite|SetFlipbook _sprite "/Game/Textures/Droids/GhostBot/Flipbooks/FB_Owlet_Monster_Idle.FB_Owlet_Monster_Idle")))))

(event EventBeginPlay
  (EventDispatchers|BindEventtoOnDeath (EventDispatchers|CreateEvent :!event OnDie)))

(event EventTick
  (params (DeltaSeconds :type Float%20%28single-precision%29))
  (CallFunction|HandleAnimation)
  (if (or (Utility|CanSeePlayer) (not (Class|MechPaperDroid|CanAttack)))
    (Attack|HauntPlayer)))

(fn ConstructionScript)

(fn OnDie
  (Actor|DestroyActor))

(fn HauntPlayer
  (bind _sprite (Variables|Default|GetSprite))
  (bind _asmech_paper_player (Utilities|Casting|CastToMechPaperPlayer (Game|Player|GetPlayerPawn 0)))
  (if (Class|MechPaperDroid|IsAlive _asmech_paper_player)
    (if (Class|MechPaperDroid|CanAttack)
      (LocalVariables|SetLocalDirection (Math|Vector|GetUnitDirection(Vector) (Transformation|GetActorLocation) (Transformation|GetActorLocation _asmech_paper_player)))
      (Utilities|FlowControl|Sequence
        (:then_0
          ;[1 1 1] Hacky way to set character mesh based on direction it's facing
          (Math|Float|CompareFloat (- (.Yaw (Math|Vector|GetYawPitchfromVector (LocalVariables|GetLocalDirection))) 5e+01) 0.0
            (:>
              (Transformation|SetWorldRotation _sprite (Math|Rotator|MakeRotator 0.0 0.0 1.8e+02) false false))
            (:<
              (Transformation|SetWorldRotation _sprite (Math|Rotator|MakeRotator 0.0 0.0 0.0) false false))))
        (:then_1
          (Pawn|Input|AddMovementInput (LocalVariables|GetLocalDirection) 1.0 false)))
      (else
        (Pawn|Input|AddMovementInput (Math|Vector|GetForwardVector (Transformation|GetWorldRotation (Variables|Default|GetSprite))) 0.25 false)))))

(fn CanSeePlayer
  (LocalVariables|SetLocalPlayer (Game|Player|GetPlayerPawn 0))
  (LocalVariables|SetLocalSelfLocation (Transformation|GetActorLocation))
  (LocalVariables|SetLocalPlayerLocation (Transformation|GetActorLocation (LocalVariables|GetLocalPlayer)))
  (if (<= (Math|Vector|Distance(Vector) (LocalVariables|GetLocalSelfLocation) (LocalVariables|GetLocalPlayerLocation)) (Variables|Config|GetSearchRange))
    (bind _outhit (Collision|LineTraceForObjects (LocalVariables|GetLocalSelfLocation) (LocalVariables|GetLocalPlayerLocation) (Utilities|Array|MakeArray "ObjectTypeQuery3") false (Utilities|Array|MakeArray self) "None"))
    (return (== (.HitActor (Collision|BreakHitResult _outhit)) (LocalVariables|GetLocalPlayer)))))