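; BP_Door is a boss-arena door that starts the boss fight when BP_MechPaperPlayer overlaps its detection trigger.
; The overlap starts suspense on the player, plays a sound and closes every BP_Door in the level, playing their animations, enabling blocking and disabling their triggers.
; After a short delay it spawns BP_Boss offset horizontally from the player toward the trigger, with yaw chosen by side, then starts the fight.
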(event OnComponentBeginOverlap(PlayerDetection)
  (params (OverlappedComponent :type Primitive%20Component%20Object%20Reference) (OtherActor :type Actor%20Object%20Reference) (OtherComp :type Primitive%20Component%20Object%20Reference) (OtherBodyIndex :type Integer) (bFromSweep :type Boolean) (SweepResult :type Hit%20Result%20Structure%20%28by%20ref%29))
  (bind _asbp_mech_paper_player (Utilities|Casting|CastToBP_MechPaperPlayer OtherActor))
  (Default|CallStartSuspense _asbp_mech_paper_player)
  (bind _outactors (Actor|GetAllActorsOfClass "BP_Door_C"))
  (for _array_element _outactors
    (Interact|CloseDoors _array_element))
  (Audio|SpawnSoundatLocation "/Game/Sound/SFX/8bit_digital_interference_2.8bit_digital_interference_2" (Transformation|GetActorLocation) "0, 0, 0" 0.7 1.0 0.0 0 0)
  (Utilities|FlowControl|Delay 2.5)
  (Interact|SpawnBoss _asbp_mech_paper_player)
  (Default|CallStartBossFight _asbp_mech_paper_player))

(event EventBeginPlay
  (bind _rendercomponent (Variables|Default|GetRenderComponent))
  (Audio|Components|Audio|Stop _rendercomponent)
  (Components|Timeline|SetLooping _rendercomponent false)
  (Class|PaperFlipbookComponent|SetPlaybackPositioninFrames _rendercomponent 0 false))

(fn ConstructionScript)

(fn CloseDoors
  (bind _doorcollision (Variables|Default|GetDoorCollision))
  (Components|Timeline|PlayfromStart (Variables|Default|GetRenderComponent))
  (Collision|SetCollisionEnabled _doorcollision "QueryOnly")
  (Collision|SetCollisionResponsetoAllChannels _doorcollision "ECR_Block")
  (Collision|SetCollisionEnabled (Variables|Default|GetPlayerDetection) "NoCollision"))

(fn SpawnBoss
  (params (Player :type Mech%20Paper%20Player%20Object%20Reference))
  (LocalVariables|SetLocalPlayerLocation (Transformation|GetActorLocation Player))
  (LocalVariables|SetLocalDetectionLocation (Transformation|GetWorldLocation (Variables|Default|GetPlayerDetection)))
  (LocalVariables|SetLocalDirection (>= (.x (Math|Vector|GetUnitDirection(Vector) (LocalVariables|GetLocalDetectionLocation) (LocalVariables|GetLocalPlayerLocation))) 0.0))
  (Game|SpawnActorfromClass "/Game/Blueprints/Enemies/BP_Boss.BP_Boss_C" (Math|Transform|MakeTransform (Math|Vector|MakeVector (+ (.x (LocalVariables|GetLocalPlayerLocation)) (* 1.1e+02 (Math|Float|SelectFloat -1.0 1.0 (LocalVariables|GetLocalDirection)))) (.y (LocalVariables|GetLocalPlayerLocation)) (.z (LocalVariables|GetLocalDetectionLocation))) (Math|Rotator|MakeRotator 0.0 0.0 (Math|Float|SelectFloat 1.8e+02 0.0 (LocalVariables|GetLocalDirection))) "1.000000,1.000000,1.000000") "AdjustIfPossibleButAlwaysSpawn" 0 0))