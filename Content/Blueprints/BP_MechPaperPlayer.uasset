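; Player-controlled chibi robot Paper2D character for a side-scroller, with movement, jumping, three-slot weapon swapping and main or special attacks.
; Tick picks idle, run or jump flipbooks; attacks use cooldown delays, and specials start looping energy recharge.
; TickAnimations gates animation, jumping and attacks, switched off with movement for hurt, death and win reactions.
; Hurt recovery uses timers for brief invincibility; winning saves and returns to the main menu.
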(event Custom|HandleAnimation
  (bind _sprite (Variables|Default|GetSprite))
  (bind _charactermovement (Variables|Character|GetCharacterMovement))
  (if (AI|Components|NavMovement|IsFalling _charactermovement)
    (Sprite|SetFlipbook _sprite "/Game/Textures/Droids/chibi-robot/chibi-robot_files/jump/FB_chibi-robot_jump.FB_chibi-robot_jump")
    (elif (> (Math|Vector|VectorLength (Variables|/Script/Engine.MovementComponent|GetVelocity _charactermovement)) 0.0)
      (Sprite|SetFlipbook _sprite "/Game/Textures/Droids/chibi-robot/chibi-robot_files/run/FB_Chibi-Robot_Run.FB_Chibi-Robot_Run")
      (else
        (Sprite|SetFlipbook _sprite "/Game/Textures/Droids/chibi-robot/chibi-robot_files/idle/FB_Chibi-Robot_Idle.FB_Chibi-Robot_Idle")))))

(event Custom|RechargeEnergy
  (Class|MechPaperPlayer|RegainEnergy (Variables|Default|GetRechargeEnergyRate)))

(event Custom|OnWin
  (Utility|DisableTickAnimations)
  (Sprite|SetFlipbook (Variables|Default|GetSprite) "/Game/Textures/Droids/chibi-robot/chibi-robot-extended-files/Sprites/victory/FB_chibi-robot-victory.FB_chibi-robot-victory")
  (Class|MechPaperPlayer|SaveonWin)
  (Utilities|FlowControl|Delay 5.5)
  (Game|OpenLevel(byName) "Map_MainMenu"))

(event EventBeginPlay
  (Initialize|BindEvents))

(event EventTick
  (params (DeltaSeconds :type Float%20%28single-precision%29))
  (if (Variables|Default|GetTickAnimations)
    (CallFunction|HandleAnimation)))

(event Input|ActionEvents|InputActionJump
  (params (Key :type Key%20Structure))
  (:Pressed
    (if (Variables|Default|GetTickAnimations)
      (Character|Jump)))
  (:Released
    (Character|StopJumping)))

(event Input|ActionEvents|InputActionFireWeapon
  (params (Key :type Key%20Structure))
  (:Pressed
    (if (Variables|Default|GetTickAnimations)
      (bind _returnvalue (Class|MechPaperPlayer|ActivateEquippedWeaponMain))
      (if _returnvalue
        (Class|MechPaperDroid|SetCanAttack false)
        (Utilities|FlowControl|Delay (Class|MechPaperPlayer|GetEquippedWeaponCooldown))
        (Class|MechPaperDroid|SetCanAttack true)))))

(event Input|ActionEvents|InputActionFireWeaponSpecial
  (params (Key :type Key%20Structure))
  (:Pressed
    (if (Variables|Default|GetTickAnimations)
      (bind _returnvalue (Class|MechPaperPlayer|ActivateEquippedWeaponSpecial))
      (if _returnvalue
        (Utilities|Time|SetTimerbyEvent (delegate Custom|RechargeEnergy) (Variables|Default|GetRechargeEnergyTimer) true)
        (Class|MechPaperDroid|SetCanAttack false)
        (Utilities|FlowControl|Delay (* (Class|MechPaperPlayer|GetEquippedWeaponCooldown) 1.5))
        (Class|MechPaperDroid|SetCanAttack true)))))

(event Input|AxisEvents|InputAxisMoveRight
  (params (AxisValue :type Float%20%28single-precision%29))
  (bind _returnvalue (Pawn|GetController))
  (if (Utilities|Enum|NotEqual(Enum) (Variables|/Script/Engine.CharacterMovementComponent|GetMovementMode (Variables|Character|GetCharacterMovement)) "MOVE_None")
    (Pawn|Input|AddMovementInput "1.000000, 0, 0" AxisValue false)
    (Math|Float|CompareFloat AxisValue 0.0
      (:>
        (Pawn|SetControlRotation _returnvalue (Math|Rotator|MakeRotator 0.0 0.0 0.0)))
      (:<
        (Pawn|SetControlRotation _returnvalue (Math|Rotator|MakeRotator 0.0 0.0 1.8e+02))))))

(event Input|KeyboardEvents|1
  (params (Key :type Key%20Structure))
  (:Pressed
    (Class|MechPaperPlayer|SwapEquippedWeapon)))

(event Input|KeyboardEvents|2
  (params (Key :type Key%20Structure))
  (:Pressed
    (Class|MechPaperPlayer|SwapEquippedWeapon 1)))

(event Input|KeyboardEvents|3
  (params (Key :type Key%20Structure))
  (:Pressed
    (Class|MechPaperPlayer|SwapEquippedWeapon 2)))

(fn ConstructionScript)

(fn BindEvents
  (EventDispatchers|BindEventtoOnHealthUpdated (EventDispatchers|CreateEvent :!event OnTakeDamage))
  (EventDispatchers|BindEventtoOnDeath (EventDispatchers|CreateEvent :!event OnPlayerDeath))
  (EventDispatchers|BindEventtoWin (EventDispatchers|CreateEvent :!event OnWin)))

(fn OnTakeDamage
  (params (NewPercent :type Float%20%28single-precision%29))
  (if (> NewPercent 0.0)
    (Sprite|SetFlipbook (Variables|Default|GetSprite) "/Game/Textures/Droids/chibi-robot/chibi-robot_files/hurt/FB_Chibi-Robot_Hurt.FB_Chibi-Robot_Hurt")
    (Audio|SpawnSound2D "/Game/Sound/SFX/8bit_destroy_1.8bit_destroy_1" 0.7 1.3 0.0 0)
    (Utility|DisableTickAnimations)
    (Utilities|Time|SetTimerbyFunctionName 0 "EnableTickAnimations" 1.05)))

(fn DisableInvincibilityFrames
  (Class|MechPaperDroid|SetCanbeDamaged true))

(fn DisableTickAnimations
  (bind _charactermovement (Variables|Character|GetCharacterMovement))
  (Collision|SetCollisionEnabled (Variables|Default|GetCapsuleComponent) "PhysicsOnly")
  (Variables|Default|SetTickAnimations false)
  (Class|MechPaperDroid|SetCanbeDamaged false)
  (Class|NavMovementComponent|StopActiveMovement _charactermovement)
  (Pawn|Components|CharacterMovement|SetMovementMode _charactermovement "MOVE_None" 0))

(fn EnableTickAnimations
  (Variables|Default|SetTickAnimations true)
  (Collision|SetCollisionEnabled (Variables|Default|GetCapsuleComponent) "QueryAndPhysics")
  (Pawn|Components|CharacterMovement|SetMovementMode (Variables|Character|GetCharacterMovement) "MOVE_Walking" 0)
  (Utilities|Time|SetTimerbyFunctionName 0 "DisableInvincibilityFrames" 0.5))

(fn OnPlayerDeath
  (bind _sprite (Variables|Default|GetSprite))
  (Collision|SetCollisionEnabled (Variables|Default|GetCapsuleComponent) "NoCollision")
  (Utilities|Time|ClearTimerbyFunctionName 0 "EnableTickAnimations")
  (Utility|DisableTickAnimations)
  (Components|Timeline|SetLooping _sprite false)
  (Sprite|SetFlipbook _sprite "/Game/Textures/Droids/chibi-robot/chibi-robot-extended-files/Sprites/crouch/FB_Chibi-Robot_Death.FB_Chibi-Robot_Death")
  (Audio|PlaySound2D "/Game/Sound/Music/Raw/xDeviruchi_-_Title_Theme_.xDeviruchi_-_Title_Theme_" 1.0 0.6 0.0 0 0))