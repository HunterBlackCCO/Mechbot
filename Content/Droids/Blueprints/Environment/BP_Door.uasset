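; BP_Door is a flipbook door that triggers the boss encounter when the player overlaps its detection volume.
; The overlap starts the player's suspense state, closes every BP_Door in the level and plays an interference sound.
; Closing plays the animation, enables blocking collision and disables detection.
; After a delay it spawns BP_Boss, halfway between player and trigger along X, and starts the player's boss fight.
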(event OnComponentBeginOverlap(PlayerDetection)
  (params (OverlappedComponent :type Primitive%20Component%20Object%20Reference) (OtherActor :type Actor%20Object%20Reference) (OtherComp :type Primitive%20Component%20Object%20Reference) (OtherBodyIndex :type Integer) (bFromSweep :type Boolean) (SweepResult :type Hit%20Result%20Structure%20%28by%20ref%29))
  (bind _asbp_mech_paper_player (Utilities|Casting|CastToBP_MechPaperPlayer OtherActor))
  (Default|CallStartSuspense _asbp_mech_paper_player)
  (bind _outactors (Actor|GetAllActorsOfClass "BP_Door_C"))
  (for _array_element _outactors
    (CallFunction|CloseDoors _array_element))
  (Audio|SpawnSoundatLocation "/Game/Sound/SFX/Game_Jingles_and_8-Bit_Sound_FX/Misc/8bit_digital_interference_2.8bit_digital_interference_2" (Transformation|GetActorLocation) "0, 0, 0" 0.7 1.0 0.0 0 0)
  (Utilities|FlowControl|Delay 2.5)
  (CallFunction|SpawnBoss _asbp_mech_paper_player)
  (Default|CallStartBossFight _asbp_mech_paper_player))

(event EventBeginPlay
  (bind _rendercomponent (Variables|Default|GetRenderComponent))
  (Audio|Components|Audio|Stop _rendercomponent)
  (Components|Timeline|SetLooping _rendercomponent false)
  (Class|PaperFlipbookComponent|SetPlaybackPositioninFrames _rendercomponent 0 false))

(fn ConstructionScript)

(fn SpawnBoss
  (params (Player :type Mech%20Paper%20Player%20Object%20Reference))
  (bind _playerdetection (Variables|Default|GetPlayerDetection))
  (bind _returnvalue (Transformation|GetWorldLocation _playerdetection))
  (LocalVariables|SetLocalLocation (Transformation|GetActorLocation Player))
  (Game|SpawnActorfromClass "/Game/Droids/Blueprints/Enemies/BP_Boss.BP_Boss_C" (Math|Transform|MakeTransform (Math|Vector|MakeVector (/ (+ (.x (LocalVariables|GetLocalLocation)) (.x _returnvalue)) 2.0) (.y (LocalVariables|GetLocalLocation)) (.z _returnvalue)) "0, 0, 0" "1.000000,1.000000,1.000000") "AdjustIfPossibleButAlwaysSpawn" 0 0))

(fn CloseDoors
  (bind _doorcollision (Variables|Default|GetDoorCollision))
  (Components|Timeline|PlayfromStart (Variables|Default|GetRenderComponent))
  (Collision|SetCollisionEnabled _doorcollision "QueryOnly")
  (Collision|SetCollisionResponsetoAllChannels _doorcollision "ECR_Block")
  (Collision|SetCollisionEnabled (Variables|Default|GetPlayerDetection) "NoCollision"))