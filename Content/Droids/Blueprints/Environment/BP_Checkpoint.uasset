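; Checkpoint actor that saves the Mech paper player's progress when that player overlaps its hitbox.
; An inactive checkpoint calls SaveProgress, plays a low-pitched activation sound and switches its flipbook to the closed idle through Close.
; OnInitialize applies the same closed look if the checkpoint is already active.
; BeginPlay binds save and creation events, while a test branch for loading the save slot is left unconnected.
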(event OnComponentBeginOverlap(Hitbox)
  (params (OverlappedComponent :type Primitive%20Component%20Object%20Reference) (OtherActor :type Actor%20Object%20Reference) (OtherComp :type Primitive%20Component%20Object%20Reference) (OtherBodyIndex :type Integer) (bFromSweep :type Boolean) (SweepResult :type Hit%20Result%20Structure%20%28by%20ref%29))
  (bind _activationsfx (Variables|Default|GetActivationSFX))
  (bind _asmech_paper_player (Utilities|Casting|CastToMechPaperPlayer OtherActor))
  (if (not (Class|MechCheckpoint|IsCheckpointActive))
    (Class|MechCheckpoint|SaveProgress _asmech_paper_player)
    (Utilities|IsValid _activationsfx
      (:Is%20Valid
        (Audio|SpawnSound2D _activationsfx 0.7 0.2 0.0 0))
      (:Is%20Not%20Valid
        _))
    (Event|Close)))

(event EventBeginPlay
  (EventDispatchers|BindEventtoOnSave (EventDispatchers|CreateEvent :!event Close))
  (EventDispatchers|BindEventtoOnCreated (EventDispatchers|CreateEvent :!event OnInitialize)))

(fn ConstructionScript)

(fn Close
  (Sprite|SetFlipbook (Variables|Default|GetSprite) "/Game/Textures/Sci-Fi_Platformer_Assets/Sci-Fi_Platformer_Prop_Pack/Sci-Fi_Platformer_Prop_Pack/1_save_point_64x64/FB_SavePoint_Idle_Close.FB_SavePoint_Idle_Close"))

(fn OnInitialize
  (if (Class|MechCheckpoint|IsCheckpointActive)
    (Event|Close)))