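; BP_MechPaperPlayer is a Paper2D side-scrolling player character: a chibi robot that runs along X, jumps and turns by flipping controller yaw.
; Tick picks idle, run or jump flipbooks from movement state, gated by TickAnimations.
; Bound health events play hurt, briefly disabling movement, damage and collision queries until a timer restores them.
; Death cancels that timer, disables the character, plays a non-looping death flipbook and starts a music track.
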(event Custom|HandleAnimation
  (bind _sprite (Variables|Default|GetSprite))
  (bind _charactermovement (Variables|Character|GetCharacterMovement))
  (if (AI|Components|NavMovement|IsFalling _charactermovement)
    (Sprite|SetFlipbook _sprite "/Game/Droids/chibi-robot/chibi-robot_files/jump/FB_chibi-robot_jump.FB_chibi-robot_jump")
    (elif (> (Math|Vector|VectorLength (Variables|/Script/Engine.MovementComponent|GetVelocity _charactermovement)) 0.0)
      (Sprite|SetFlipbook _sprite "/Game/Droids/chibi-robot/chibi-robot_files/run/FB_Chibi-Robot_Run.FB_Chibi-Robot_Run")
      (else
        (Sprite|SetFlipbook _sprite "/Game/Droids/chibi-robot/chibi-robot_files/idle/FB_Chibi-Robot_Idle.FB_Chibi-Robot_Idle")))))

(event EventBeginPlay
  (Initialize|BindEvents))

(event EventTick
  (params (DeltaSeconds :type Float%20%28single-precision%29))
  (if (Variables|Default|GetTickAnimations)
    (CallFunction|HandleAnimation)))

(event Input|ActionEvents|InputActionJump
  (params (Key :type Key%20Structure :default "None"))
  (:Pressed
    (if (Variables|Default|GetTickAnimations)
      (Character|Jump)))
  (:Released
    (Character|StopJumping)))

(event Input|ActionEvents|InputActionFireWeapon
  (params (Key :type Key%20Structure :default "None")))

(event Input|ActionEvents|InputActionFireWeaponSpecial
  (params (Key :type Key%20Structure :default "None")))

(event Input|AxisEvents|InputAxisMoveRight
  (params (AxisValue :type Float%20%28single-precision%29))
  (bind _returnvalue (Pawn|GetController))
  (if (Utilities|Enum|NotEqual(Enum) (Variables|/Script/Engine.CharacterMovementComponent|GetMovementMode (Variables|Character|GetCharacterMovement)) "MOVE_None")
    (Pawn|Input|AddMovementInput "1.000000, 0, 0" AxisValue false)
    (Math|Float|CompareFloat AxisValue 0.0
      (:>
        (Pawn|SetControlRotation _returnvalue (Math|Rotator|MakeRotator 0.0 0.0 0.0)))
      (:<
        (Pawn|SetControlRotation _returnvalue (Math|Rotator|MakeRotator 0.0 0.0 1.8e+02))))))

(fn ConstructionScript)

(fn BindEvents
  (EventDispatchers|BindEventtoOnHealthUpdated (EventDispatchers|CreateEvent :!event OnTakeDamage))
  (EventDispatchers|BindEventtoOnDeath (EventDispatchers|CreateEvent :!event OnPlayerDeath)))

(fn OnTakeDamage
  (params (NewPercent :type Float%20%28single-precision%29))
  (if (> NewPercent 0.0)
    (Sprite|SetFlipbook (Variables|Default|GetSprite) "/Game/Droids/chibi-robot/chibi-robot_files/hurt/FB_Chibi-Robot_Hurt.FB_Chibi-Robot_Hurt")
    (Utility|DisableTickAnimations)
    (Utilities|Time|SetTimerbyFunctionName 0 "EnableTickAnimations" 1.5)))

(fn DisableTickAnimations
  (bind _charactermovement (Variables|Character|GetCharacterMovement))
  (Collision|SetCollisionEnabled (Variables|Default|GetCapsuleComponent) "PhysicsOnly")
  (Variables|Default|SetTickAnimations false)
  (Variables|Default|SetbCanBeDamaged false)
  (Class|NavMovementComponent|StopActiveMovement _charactermovement)
  (Pawn|Components|CharacterMovement|SetMovementMode _charactermovement "MOVE_None" 0))

(fn EnableTickAnimations
  (Variables|Default|SetTickAnimations true)
  (Variables|Default|SetbCanBeDamaged true)
  (Collision|SetCollisionEnabled (Variables|Default|GetCapsuleComponent) "QueryAndPhysics")
  (Pawn|Components|CharacterMovement|SetMovementMode (Variables|Character|GetCharacterMovement) "MOVE_Walking" 0))

(fn OnPlayerDeath
  (bind _sprite (Variables|Default|GetSprite))
  (Collision|SetCollisionEnabled (Variables|Default|GetCapsuleComponent) "NoCollision")
  (Utilities|Time|ClearTimerbyFunctionName 0 "EnableTickAnimations")
  (Utility|DisableTickAnimations)
  (Components|Timeline|SetLooping _sprite false)
  (Sprite|SetFlipbook _sprite "/Game/Droids/chibi-robot/chibi-robot-extended-files/Sprites/crouch/FB_Chibi-Robot_Death.FB_Chibi-Robot_Death")
  (Audio|PlaySound2D "/Game/Sound/Music/xDeviruchi_8-bit_Fantasy_Adventure_Music__2021_/xDeviruchi_-_Title_Theme_.xDeviruchi_-_Title_Theme_" 1.0 0.6 0.0 0 0))