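; RinoFish enemy, a 2D flipbook droid that bites players in close range and rolls at them from afar.
; A looping timer checks range and traces against pawns, then starts a timed roll toward the player's captured position.
; While rolling it cannot be damaged, Tick drives movement and facing, and capsule overlaps deal damage.
; Bite-collision overlap swaps the search timer for a looping bite timer that damages overlapping players until overlap ends.
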(event OnComponentBeginOverlap(CapsuleComponent)
  (params (OverlappedComponent :type Primitive%20Component%20Object%20Reference) (OtherActor :type Actor%20Object%20Reference) (OtherComp :type Primitive%20Component%20Object%20Reference) (OtherBodyIndex :type Integer) (bFromSweep :type Boolean) (SweepResult :type Hit%20Result%20Structure%20%28by%20ref%29))
  (if (Variables|Cached|GetIsRolling)
    (bind _asmech_paper_player (Utilities|Casting|CastToMechPaperPlayer OtherActor))
    (Class|MechPaperDroid|TakeDamage _asmech_paper_player (Variables|Config|GetRollDamage))))

(event OnComponentBeginOverlap(BiteCollision)
  (params (OverlappedComponent :type Primitive%20Component%20Object%20Reference) (OtherActor :type Actor%20Object%20Reference) (OtherComp :type Primitive%20Component%20Object%20Reference) (OtherBodyIndex :type Integer) (bFromSweep :type Boolean) (SweepResult :type Hit%20Result%20Structure%20%28by%20ref%29))
  (Utilities|Casting|CastToMechPaperPlayer OtherActor)
  (if (not (or (Variables|Cached|GetIsBiting) (Variables|Cached|GetIsRolling)))
    (Utilities|Time|ClearTimerbyFunctionName 0 (Variables|Cached|GetSearchForPlayerFunctionName))
    (bind _returnvalue (Utilities|Time|SetTimerbyEvent (delegate Custom|Bite) 0.1 true))
    (Variables|Default|SetBiteTimer _returnvalue)))

(event OnComponentEndOverlap(BiteCollision)
  (params (OverlappedComponent :type Primitive%20Component%20Object%20Reference) (OtherActor :type Actor%20Object%20Reference) (OtherComp :type Primitive%20Component%20Object%20Reference) (OtherBodyIndex :type Integer))
  (Utilities|Casting|CastToMechPaperPlayer OtherActor)
  (if (not (Variables|Cached|GetIsRolling))
    (Utilities|Time|ClearandInvalidateTimerbyHandle (Variables|Default|GetBiteTimer))
    (Utilities|Time|SetTimerbyFunctionName 0 (Variables|Cached|GetSearchForPlayerFunctionName) 2.0 true)))

(event Custom|Bite
  (bind _sprite (Variables|Default|GetSprite))
  (bind _sprite_2 (Variables|Default|GetSprite))
  (Variables|Cached|SetIsBiting true)
  (Sprite|SetFlipbook _sprite_2 "/Game/Droids/Warped_Rino_Fish/rino-fish-bite/sprites/FB_Rino-Fish_Bite.FB_Rino-Fish_Bite")
  (Components|Timeline|SetLooping _sprite_2 false)
  (Attack|BitePlayer)
  (Utilities|FlowControl|Delay (Class|PaperFlipbookComponent|GetFlipbookLength _sprite_2))
  (Sprite|SetFlipbook _sprite "/Game/Droids/Warped_Rino_Fish/rino-fish-idle/sprites/FB_Rino-Fish_Idle.FB_Rino-Fish_Idle")
  (Components|Timeline|SetLooping _sprite true)
  (Audio|Components|Audio|Play _sprite)
  (Variables|Cached|SetIsBiting false))

(event EventTick
  (params (DeltaSeconds :type Float%20%28single-precision%29))
  (bind _returnvalue (Pawn|GetController))
  (bind _rollingdirection (Variables|Cached|GetRollingDirection))
  (if (Variables|Cached|GetIsRolling)
    (Pawn|Input|AddMovementInput _rollingdirection 1.0 false)
    (Math|Float|CompareFloat (.X (Math|Vector|BreakVector _rollingdirection)) 0.0
      (:>
        (Pawn|SetControlRotation _returnvalue (Math|Rotator|MakeRotator 0.0 0.0 0.0)))
      (:<
        (Pawn|SetControlRotation _returnvalue (Math|Rotator|MakeRotator 0.0 0.0 1.8e+02))))))

(event EventBeginPlay
  (Utilities|Time|SetTimerbyFunctionName 0 (Variables|Cached|GetSearchForPlayerFunctionName) 2.0 true))

(fn ConstructionScript)

(fn BitePlayer
  (bind _output_get (LocalVariables|SetLocalPlayers (Collision|GetOverlappingActors (Variables|Default|GetBiteCollision) "/Script/Mechbot.MechPaperPlayer" :!class /Script/Engine.PrimitiveComponent)))
  (for _array_element _output_get
    (bind _asmech_paper_player (Utilities|Casting|CastToMechPaperPlayer _array_element))
    (Class|MechPaperDroid|TakeDamage _asmech_paper_player (Variables|Config|GetBiteDamage))))

(fn StartRolling
  (Sprite|SetFlipbook (Variables|Default|GetSprite) "/Game/Droids/Warped_Rino_Fish/rino-fish-rolling/sprites/FB_Rino-Fish_Rolling.FB_Rino-Fish_Rolling")
  (Variables|Default|SetbCanBeDamaged false)
  (Variables|Cached|SetIsRolling true)
  (Variables|Cached|SetRollingDirection (Math|Vector|GetUnitDirection(Vector) (Transformation|GetActorLocation) (Transformation|GetActorLocation (Game|Player|GetPlayerPawn 0))))
  (Utilities|Time|SetTimerbyFunctionName 0 "StopRolling" 2.0))

(fn StopRolling
  (Class|NavMovementComponent|StopActiveMovement (Variables|Character|GetCharacterMovement))
  (Sprite|SetFlipbook (Variables|Default|GetSprite) "/Game/Droids/Warped_Rino_Fish/rino-fish-idle/sprites/FB_Rino-Fish_Idle.FB_Rino-Fish_Idle")
  (Variables|Cached|SetIsRolling false)
  (Variables|Default|SetbCanBeDamaged true))

(fn SearchforPlayer
  (if (Math|Boolean|NORBoolean (Variables|Cached|GetIsBiting) (Variables|Cached|GetIsRolling))
    (LocalVariables|SetLocalPlayer (Game|Player|GetPlayerPawn 0))
    (LocalVariables|SetLocalSelfLocation (Transformation|GetActorLocation))
    (LocalVariables|SetLocalPlayerLocation (Transformation|GetActorLocation (LocalVariables|GetLocalPlayer)))
    (if (<= (Math|Vector|Distance(Vector) (LocalVariables|GetLocalSelfLocation) (LocalVariables|GetLocalPlayerLocation)) (Variables|Config|GetSearchRange))
      (bind _outhit (Collision|LineTraceForObjects (LocalVariables|GetLocalSelfLocation) (LocalVariables|GetLocalPlayerLocation) (Utilities|Array|MakeArray "ObjectTypeQuery3") false (Utilities|Array|MakeArray self) "None"))
      (if (== (.HitActor (Collision|BreakHitResult _outhit)) (LocalVariables|GetLocalPlayer))
        (Attack|StartRolling)))))