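; BP_GhostBot is a flipbook-animated enemy that chases the player's MechPaperPlayer and damages it on capsule overlap.
; Each Tick it steers directly along the vector to the living player, creeping closer while the player can be damaged and backing away at full input otherwise.
; Tick also picks the Owlet Monster jump, walk or idle flipbook from the movement state.
; A BT_GhostBot behavior tree launch exists but is unconnected and never runs.
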(event OnComponentBeginOverlap(CapsuleComponent)
  (params (OverlappedComponent :type Primitive%20Component%20Object%20Reference) (OtherActor :type Actor%20Object%20Reference) (OtherComp :type Primitive%20Component%20Object%20Reference) (OtherBodyIndex :type Integer) (bFromSweep :type Boolean) (SweepResult :type Hit%20Result%20Structure%20%28by%20ref%29))
  (bind _asmech_paper_player (Utilities|Casting|CastToMechPaperPlayer OtherActor))
  (Class|MechPaperDroid|TakeDamage _asmech_paper_player 20))

(event Custom|HandleAnimation
  (bind _sprite (Variables|Default|GetSprite))
  (bind _charactermovement (Variables|Character|GetCharacterMovement))
  (if (AI|Components|NavMovement|IsFalling _charactermovement)
    (Sprite|SetFlipbook _sprite "/Game/Droids/free-pixel-art-tiny-hero-sprites/2_Owlet_Monster/FB_Owlet_Monster_Jump.FB_Owlet_Monster_Jump")
    (elif (> (Math|Vector|VectorLength (Variables|/Script/Engine.MovementComponent|GetVelocity _charactermovement)) 0.0)
      (Sprite|SetFlipbook _sprite "/Game/Droids/free-pixel-art-tiny-hero-sprites/2_Owlet_Monster/FB_Owlet_Monster_Walk.FB_Owlet_Monster_Walk")
      (else
        (Sprite|SetFlipbook _sprite "/Game/Droids/free-pixel-art-tiny-hero-sprites/2_Owlet_Monster/FB_Owlet_Monster_Idle.FB_Owlet_Monster_Idle")))))

(event EventBeginPlay)

(event EventTick
  (params (DeltaSeconds :type Float%20%28single-precision%29))
  (CallFunction|HandleAnimation)
  (bind _asmech_paper_player (Utilities|Casting|CastToMechPaperPlayer (Game|Player|GetPlayerPawn 0)))
  (if (Class|MechPaperDroid|IsAlive _asmech_paper_player)
    (Pawn|Input|AddMovementInput (Math|Vector|GetUnitDirection(Vector) (Transformation|GetActorLocation) (Transformation|GetActorLocation _asmech_paper_player)) (Math|Float|SelectFloat 0.1 -1.0 (Class|MechPaperDroid|CanbeDamaged _asmech_paper_player)) false)))

(fn ConstructionScript)